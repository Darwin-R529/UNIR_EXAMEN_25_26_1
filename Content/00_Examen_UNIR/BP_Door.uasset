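; BP_Door is a double sliding door that opens once all of its linked buttons are active.
; On BeginPlay it stores both panels' starting positions and binds Verification to each button's OnPressChanged event.
; Verification checks every button's BTNActivated state and calls OpenDoor, whose Timeline lerps the panels apart along local X.
; OpenDoor can reverse the Timeline, but Verification never requests closing.
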(event Custom|OpenDoor
  (params (Open :type Boolean))
  (if Open
    (bind _newtrack_0 (Timeline|Timeline Play)
      (:Update
        (Transformation|SetRelativeLocation (Variables|Default|GetRigthDoor) (Math|Vector|Lerp(Vector) (Variables|Default|GetInitPos_RigthDoor) (+ (Variables|Default|GetInitPos_RigthDoor) "80.000000,0.000000,0.000000") _newtrack_0) false false)
        (Transformation|SetRelativeLocation (Variables|Default|GetLeftDoor) (Math|Vector|Lerp(Vector) (Variables|Default|GetInitPos_LeftDoor) (+ (Variables|Default|GetInitPos_LeftDoor) "-80.000000,0.000000,0.000000") _newtrack_0) false false)))
    (else
      (Timeline|Timeline Reverse))))

(event Custom|Verification
  (Variables|Default|SetAreAllBTNActive true)
  (for _array_element (Variables|Default|Getbuttons)
    (if (not (Variables|/Game/00_Examen_UNIR/BP_FloorButton.BP_FloorButton_C|GetBTNActivated _array_element))
      (Variables|Default|SetAreAllBTNActive false)))
  (if (Variables|Default|GetAreAllBTNActive)
    (CallFunction|OpenDoor true)))

(event EventBeginPlay
  (Variables|Default|SetInitPos_RigthDoor (Variables|/Script/Engine.SceneComponent|GetRelativeLocation (Variables|Default|GetRigthDoor)))
  (Variables|Default|SetInitPos_LeftDoor (Variables|/Script/Engine.SceneComponent|GetRelativeLocation (Variables|Default|GetLeftDoor)))
  (for _array_element (Variables|Default|Getbuttons)
    (EventDispatchers|BindEventtoOnPressChanged _array_element (delegate Custom|Verification))))

(event Collision|EventActorBeginOverlap
  (params (OtherActor :type Actor%20Object%20Reference)))

(event EventTick
  (params (DeltaSeconds :type Float%20%28single-precision%29)))

(fn ConstructionScript)